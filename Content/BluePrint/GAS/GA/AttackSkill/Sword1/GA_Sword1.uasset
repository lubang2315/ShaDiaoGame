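; GA_Sword1 is a Gameplay Ability for a mouse-targeted sword attack skill.
; On activation it starts capturing the mouse hit location, then after a short delay waits for an input press to lock the target.
; The press replaces any existing sword with a newly spawned one and activates its ability toward that point.
; When the sword reports a successful move, it applies sphere damage there and ends the ability after a delay.
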(event `self.K2_ActivateAbility`
  (bind _mousehitpointlocation (`self.MouseHitPointLocation`))
  (`self.StartCaptureMouseHitLocation`)
  (`KismetSystemLibrary.Delay` 0.2)
  (`AbilityTask_WaitInputPress.WaitInputPress` false
    (:`OnPress`
      (`self.EndCaptureMouseHitLocation`)
      (`self.DestorySword`)
      (set `self.HitSourceLocation` _mousehitpointlocation)
      (`self.SpawnSwordAndActiveGA` _mousehitpointlocation)
      (bind _sword (`self.Sword`)
        (:`then`
          (add `Actor_Sword.OnMoveDone` _sword (delegate `OnMoveDone_事件`)))
        (:`else`)))))

(event `OnMoveDone_事件`
  (params (bSuccess :type Boolean))
  (if bSuccess
    (`self.SpawnSphereAndApplyDamage` (`self.MouseHitPointLocation`))
    (`KismetSystemLibrary.Delay` 2.0)
    (`self.EndSwordAbility`)
    (`self.K2_EndAbility`)))