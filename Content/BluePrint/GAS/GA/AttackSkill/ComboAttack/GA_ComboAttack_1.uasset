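; Gameplay Ability for an axe-and-shield melee combo that chains up to four attack montages (A to D).
; A TestTag gameplay event opens or closes the input window by magnitude; a press inside it sets IsPlayCombo1.
; Each completed montage checks that flag to play the next attack or end the ability.
; In parallel, sword collision events call OnSwordCollisioncomponents by magnitude and record the avatar's location as HitSourceLocation.
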(event `self.K2_ActivateAbility`
  (`|ExecutionSequence`
    (:`then_0`
      (bind (_asynctaskproxy _payload) (`AbilityTask_WaitGameplayEvent.WaitGameplayEvent` (struct :`TagName` "Event.Sword.Collision") null)
        (:`EventReceived`
          (`self.OnSwordCollisioncomponents` (> (`.EventMagnitude` (break `GameplayEventData` _payload)) 0.0))
          (set `self.HitSourceLocation` (`Actor.K2_GetActorLocation` (`self.GetAvatarActorFromActorInfo`))))))
    (:`then_1`
      (`AbilityTask_PlayMontageAndWait.CreatePlayMontageAndWaitProxy` "None" "/Game/Asset/UserAsset/Player/Animoation/Player/Combot/AxeAndShield_Attack_A_Montage1.AxeAndShield_Attack_A_Montage1" 0.8
        (:`then`
          (bind (_asynctaskproxy_2 _payload_2) (`AbilityTask_WaitGameplayEvent.WaitGameplayEvent` (struct :`TagName` "TestTag") null)
            (:`EventReceived`
              (bind _output_get (set `self.IsTiming` (> (`.EventMagnitude` (break `GameplayEventData` _payload_2)) 0.0)))
              (if _output_get
                (`AbilityTask_WaitInputPress.WaitInputPress` false
                  (:`OnPress`
                    (set `self.IsPlayCombo1` true)))
                (else
                  (set `self.IsPlayCombo1` false))))))
        (:`OnCompleted`
          (if (`self.IsPlayCombo1`)
            (`AbilityTask_PlayMontageAndWait.CreatePlayMontageAndWaitProxy` "None" "/Game/Asset/UserAsset/Player/Animoation/Player/Combot/AxeAndShield_Attack_B_Montage1.AxeAndShield_Attack_B_Montage1" 0.8
              (:`then`
                (set `self.IsPlayCombo1` false))
              (:`OnCompleted`
                (if (`self.IsPlayCombo1`)
                  (`AbilityTask_PlayMontageAndWait.CreatePlayMontageAndWaitProxy` "None" "/Game/Asset/UserAsset/Player/Animoation/Player/Combot/AxeAndShield_Attack_C_Montage1.AxeAndShield_Attack_C_Montage1" 0.8
                    (:`then`
                      (set `self.IsPlayCombo1` false))
                    (:`OnCompleted`
                      (if (`self.IsPlayCombo1`)
                        (`AbilityTask_PlayMontageAndWait.CreatePlayMontageAndWaitProxy` "None" "/Game/Asset/UserAsset/Player/Animoation/Player/Combot/AxeAndShield_Attack_D_Montage.AxeAndShield_Attack_D_Montage" 0.8
                          (:`OnCompleted`
                            _)
                          (:`OnBlendOut`
                            _)
                          (:`OnInterrupted`
                            _)
                          (:`OnCancelled`
                            _))
                        (`self.K2_EndAbility`)
                        (else
                          (`self.K2_EndAbility`))))
                    (:`OnInterrupted`
                      (`self.K2_EndAbility` :!label _label))
                    (:`OnCancelled`
                      (goto _label)))
                  (else
                    (`self.K2_EndAbility`))))
              (:`OnInterrupted`
                (`self.K2_EndAbility` :!label _label_2))
              (:`OnCancelled`
                (goto _label_2)))
            (else
              (`self.K2_EndAbility`))))
        (:`OnInterrupted`
          (`self.K2_EndAbility` :!label _label_3))
        (:`OnCancelled`
          (goto _label_3))))))