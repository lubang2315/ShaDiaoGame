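; BP_GA_HookLock is a Gameplay Ability for a hook-style skill that moves the player to a targeted point.
; On activation it shows a crosshair and applies a camera offset, then waits a fixed delay before sampling the point.
; It marks that point with a debug sphere, sets the player location there, prints it and ends after a short delay.
; Ending the ability hides the crosshair and removes the camera offset.
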(event `self.K2_ActivateAbility`
  (`self.SetCrosshairShow`)
  (`self.ActivateCameraOffset`)
  (`KismetSystemLibrary.Delay` 2.0)
  (bind _returnvalue (`self.GetPoint`))
  (`KismetSystemLibrary.DrawDebugSphere` _returnvalue)
  (`self.SetPlayerLocation` _returnvalue)
  (`KismetSystemLibrary.PrintString` (`KismetStringLibrary.Conv_VectorToString` _returnvalue))
  (`KismetSystemLibrary.Delay` 0.6)
  (`self.K2_EndAbility`))

(event `self.K2_OnEndAbility`
  (params (bWasCancelled :type Boolean))
  (`self.SetCrosshairHide`)
  (`self.EndCameraOffset`))