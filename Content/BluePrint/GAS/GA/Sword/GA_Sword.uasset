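; GA_Sword is a Gameplay Ability that runs a timed sword-flight mode with its own camera.
; An IsMoving check on activation chooses between setting the sword's location and ending after a short delay, or starting the flight.
; The flight branch unbinds the sword, switches camera, enables movement and commits cost, then uses a fixed delay before restoring camera, stopping movement and committing cooldown.
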(event `self.K2_ActivateAbility`
  (`KismetSystemLibrary.PrintString` "Hello")
  (`self.IsMoving`)
  (if (not (`self.bIsMoving`))
    (`self.SetSwordLocation`)
    (`KismetSystemLibrary.Delay` 1.0)
    (`self.K2_EndAbility`)
    (else
      (`self.SetSwordUnbinding`)
      (`self.ActiveSwordCamera`)
      (`KismetSystemLibrary.Delay` 1.0)
      (`self.SetSwordMove` true)
      (`self.K2_CommitAbilityCost` false)
      (`KismetSystemLibrary.Delay` 10.0)
      (`self.EndSwordCamera`)
      (`self.EndGA_Sword`)
      (`self.SetSwordMove` false)
      (`self.K2_CommitAbilityCooldown` false)
      (`self.K2_EndAbility`))))