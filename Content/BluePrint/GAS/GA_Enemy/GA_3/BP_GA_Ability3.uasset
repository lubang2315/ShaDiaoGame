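; Gameplay ability for the enemy's third attack, playing a montage that motion-warps toward the player.
; StartGA sets the "root" warp target on BP_Enemy from PlayerLocation and AttackAbsorbRotation, then plays Attack_03_Montage.
; During the montage, Event.Enemy.Ability3 gameplay events start weapon collision, passing along the event magnitude.
; The ability ends when the montage completes or is cancelled.
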(event `self.StartGA`
  (bind _asbp_enemy (cast `/Game/BluePrint/Character/Enemy/Enemy_01/BP_Enemy` (`self.GetAvatarActorFromActorInfo`)))
  (`MotionWarpingComponent.AddOrUpdateWarpTargetFromLocationAndRotation` (`/Game/BluePrint/Character/Enemy/Enemy_01/BP_Enemy.MotionWarping` _asbp_enemy) "root" (`self.PlayerLocation`) (`self.AttackAbsorbRotation`))
  (`AbilityTask_PlayMontageAndWait.CreatePlayMontageAndWaitProxy` "None" "/Game/Asset/Asset_Enemy/Enemy/Animoation/Montage/attack_03_Montage.attack_03_Montage"
    (:`then`
      (bind (_asynctaskproxy _payload) (`AbilityAsync_WaitGameplayEvent.WaitGameplayEventToActor` (`self.GetAvatarActorFromActorInfo`) (struct :`TagName` "Event.Enemy.Ability3"))
        (:`EventReceived`
          (`self.StartWeaponCollision` (`.EventMagnitude` (break `GameplayEventData` _payload))))))
    (:`OnCompleted`
      (`self.K2_EndAbility` :!label _label))
    (:`OnCancelled`
      (goto _label))))