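; Enemy passive gameplay ability that plays a hit reaction montage based on the hit type.
; The first hit type picks a montage from an array indexed by hit angle.
; The second calls SetActorRotationHit, then plays a knockdown-and-rise montage.
; Both paths end the ability when the montage completes, is interrupted or is cancelled.
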(event `self.PlayHitMontag`
  (switch `int` (`self.HitType`)
    (:`0`
      (if (== (`self.HitType`) 0)
        (`AbilityTask_PlayMontageAndWait.CreatePlayMontageAndWaitProxy` "None" (`|GetArrayItem` (`self.Montage`) (`self.HitAngle`))
          (:`OnCompleted`
            _)
          (:`OnInterrupted`
            _)
          (:`OnCancelled`
            _))
        (`self.K2_EndAbility`)))
    (:`1`
      (`self.SetActorRotationHit`)
      (`AbilityTask_PlayMontageAndWait.CreatePlayMontageAndWaitProxy` "None" "/Game/Asset/Asset_Enemy/Enemy/Animoation/Montage/DownAndrise.DownAndrise"
        (:`OnCompleted`
          _)
        (:`OnInterrupted`
          _)
        (:`OnCancelled`
          _))
      (`self.K2_EndAbility`))))